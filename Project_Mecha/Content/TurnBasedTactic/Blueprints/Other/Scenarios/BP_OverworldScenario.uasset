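; Overworld scenario that sets up the map's unit groups for the turn-based tactics game and shows the back-to-main-menu widget.
; BuildUnitGroupsBasedOnUnitNames fills UnitGroups by parsing BP_Unit display names: the number after "Group" gives the group ID, "_Ai" marks an encounter.
; After a tiny delay for CharacterMovement initialization, BeginPlay sets each unit's context and registers groups and encounter flags with OverworldUnitGroupsManager.
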(event EventBeginPlay
  ;[0 0 0] [EN] Register the units in the OverworldUnitGroupsManager
  ; [FR] Passe les unités dans le OverworldUnitGroupsManager
  (bind _returnvalue (UserInterface|CreateWidget "/Game/TurnBasedTactic/Blueprints/Other/MainMenu/WBP_BackToMainMenu.WBP_BackToMainMenu_C"))
  (UserInterface|Viewport|AddtoViewport _returnvalue 0)
  (Utilities|FlowControl|Delay 0.001) ; [EN] Because CharacterMovement is not initialized on first frame for some reason\n[FR] Parce que le CharacterMovement n'est pas initialisé pendant la première frame pour une raison que j'ignore
  (bind _values (Utilities|Map|Values (Variables|Default|GetUnitGroups)))
  (for _array_element _values
    (for _array_element_2 (.Units (Utilities|Struct|BreakS_OverworldUnitGroup _array_element))
      (Default|SetUnitContext _array_element_2 "NewEnumerator1")
      (Default|AddUnittoGroup (Variables|Default|GetOverworldUnitGroupsManager) _array_element_2 (.GroupId (Utilities|Struct|BreakS_OverworldUnitGroup _array_element))))
    (Default|SetGroupIsEncounter (Variables|Default|GetOverworldUnitGroupsManager) (.IsEncounter (Utilities|Struct|BreakS_OverworldUnitGroup _array_element)) (.GroupId (Utilities|Struct|BreakS_OverworldUnitGroup _array_element)))))

(fn ConstructionScript)

(fn BuildUnitGroupsBasedonUnitNames
  ;[0 0 0] [EN] Do some string manipulations to generate the UnitGroups
  ; [FR] Fait quelques manipulations de string pour générer les UnitGroups
  (Utilities|Map|Clear (Variables|Default|GetUnitGroups))
  (bind _outactors (Actor|GetAllActorsOfClass "/Game/TurnBasedTactic/Blueprints/Core/Units/BP_Unit.BP_Unit_C"))
  (for _array_element _outactors
    (LocalVariables|SetUnit _array_element)
    (LocalVariables|SetGroupId (Math|Conversions|ToInteger(Byte) (select (.ReturnValue (Utilities|String|Split (.RightS (Utilities|String|Split (Utilities|GetDisplayName (LocalVariables|GetUnit)) "Group")) "_")) (.LeftS (Utilities|String|Split (.RightS (Utilities|String|Split (Utilities|GetDisplayName (LocalVariables|GetUnit)) "Group")) "_")) (.RightS (Utilities|String|Split (Utilities|GetDisplayName (LocalVariables|GetUnit)) "Group")))))
    (LocalVariables|SetIsEncounter (Utilities|String|Contains (Utilities|GetDisplayName (LocalVariables|GetUnit)) "_Ai"))
    (LocalVariables|SetGroup (.Value (Utilities|Map|Find (Variables|Default|GetUnitGroups) (LocalVariables|GetGroupId))))
    (Utilities|Struct|SetmembersinS_OverworldUnitGroup (LocalVariables|GetGroup) (LocalVariables|GetGroupId) (LocalVariables|GetIsEncounter))
    (Utilities|Array|AddUnique (Utilities|Struct|BreakS_OverworldUnitGroup (LocalVariables|GetGroup)) (LocalVariables|GetUnit))
    (Utilities|Map|Add (Variables|Default|GetUnitGroups) (LocalVariables|GetGroupId) (LocalVariables|GetGroup))))