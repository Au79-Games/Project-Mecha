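; Player action for the overworld that orders the currently selected unit to move to the point under the mouse cursor.
; ExecuteAction checks that a unit is selected, traces under the cursor and passes the hit location to the unit's move event.
; The hovered unit is passed along as the unit to follow, with random locations turned off.
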(event EventBeginPlay
  (|CallParentFunction) ; This node is disabled and will not be called.\nDrag off pins to build functionality.
)

(event Collision|EventActorBeginOverlap
  (params (OtherActor :type Actor%20Object%20Reference))
  (|CallParentFunction OtherActor) ; This node is disabled and will not be called.\nDrag off pins to build functionality.
)

(event EventTick
  (params (DeltaSeconds :type Float%20%28single-precision%29))
  (|CallParentFunction DeltaSeconds) ; This node is disabled and will not be called.\nDrag off pins to build functionality.
)

(fn ConstructionScript
  (|CallParentFunction))

(fn ExecuteAction
  (params (Index :type Int%20Point%20Structure))
  (bind _returnvalue (Game|GetPlayerController 0))
  (bind _playeractions (Variables|Default|GetPlayerActions))
  (bind (_hitresult _returnvalue_2) (Game|Player|GetHitResultUnderCursorbyChannel _returnvalue "TraceTypeQuery3" false))
  (bind _selectedunit (Variables|/Game/TurnBasedTactic/Blueprints/Core/Player/BP_PlayerActions.BP_PlayerActions_C|GetSelectedUnit _playeractions))
  ;[0 0 0] [EN] Ask the unit to move
  ; [FR] Demande a l'unité de marcher
  (Utilities|IsValid _selectedunit
    (:Is%20Valid
      (if _returnvalue_2
        (Default|EventMoveUnitinOverworld _selectedunit (.Location (Collision|BreakHitResult _hitresult)) (Variables|/Game/TurnBasedTactic/Blueprints/Core/Player/BP_PlayerActions.BP_PlayerActions_C|GetHoveredUnit (Variables|Default|GetPlayerActions)) false)))))