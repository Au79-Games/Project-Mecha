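; BP_Action_SetTileType is a player action that changes the type of one tile on the tactical grid.
; ExecuteAction checks that the index is valid on the Grid reached through PlayerActions, then looks up that tile's data.
; It writes the tile back through AddGridTile with the action's TileType, keeping its index, transform, states and unit.
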(fn ConstructionScript
  (|CallParentFunction))

(fn ExecuteAction
  (params (Index :type Int%20Point%20Structure))
  ;[0 0 0] [EN] We first get the Data of the existing tile. Then we replace the TileType before setting the Data back into the grid.
  ; [FR] Premièrement, on obtient le Data que la case actuelle. Puis on remplace le TileType avant de la re-set dans la grille.
  (if (Default|IsIndexValid (Variables|/Game/TurnBasedTactic/Blueprints/Core/Player/BP_PlayerActions.BP_PlayerActions_C|GetGrid (Variables|Default|GetPlayerActions)) Index)
    (LocalVariables|SetData (.Value (Utilities|Map|Find (Variables|/Game/TurnBasedTactic/Blueprints/Core/Grid/BP_Grid.BP_Grid_C|GetGridTiles (Variables|/Game/TurnBasedTactic/Blueprints/Core/Player/BP_PlayerActions.BP_PlayerActions_C|GetGrid (Variables|Default|GetPlayerActions))) Index)))
    (Default|AddGridTile (Variables|/Game/TurnBasedTactic/Blueprints/Core/Player/BP_PlayerActions.BP_PlayerActions_C|GetGrid (Variables|Default|GetPlayerActions)) (Utilities|Struct|MakeS_TileData (.Index (Utilities|Struct|BreakS_TileData (LocalVariables|GetData))) (Variables|Default|GetTileType) (.Transform (Utilities|Struct|BreakS_TileData (LocalVariables|GetData))) (.States (Utilities|Struct|BreakS_TileData (LocalVariables|GetData))) (.UnitOnTile (Utilities|Struct|BreakS_TileData (LocalVariables|GetData)))))))