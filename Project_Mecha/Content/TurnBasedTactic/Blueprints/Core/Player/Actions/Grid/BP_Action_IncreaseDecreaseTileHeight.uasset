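; Player grid action that raises or lowers the height of the targeted tile in the turn-based tactics grid.
; ExecuteAction validates the index, reads that tile's data from the grid, and shifts its transform Z by one tile-size step, up or down based on the Increase flag.
; It then writes the tile back through AddGridTile, keeping its type, rotation, scale, states and occupying unit intact.
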(fn ConstructionScript
  (|CallParentFunction))

(fn ExecuteAction
  (params (Index :type Int%20Point%20Structure))
  ;[0 0 0] [EN] We first get the Data of the existing tile. Then we Add or Substract from the current tile height befoe setting the Data back into the grid.
  ; [FR] Premièrement, on obtient le Data que la case actuelle. Puis on Ajoute ou Soustrait à partir de la hauteur courante avant de la re-set dans la grille.
  (if (Default|IsIndexValid (Variables|/Game/TurnBasedTactic/Blueprints/Core/Player/BP_PlayerActions.BP_PlayerActions_C|GetGrid (Variables|Default|GetPlayerActions)) Index)
    (LocalVariables|SetData (.Value (Utilities|Map|Find (Variables|/Game/TurnBasedTactic/Blueprints/Core/Grid/BP_Grid.BP_Grid_C|GetGridTiles (Variables|/Game/TurnBasedTactic/Blueprints/Core/Player/BP_PlayerActions.BP_PlayerActions_C|GetGrid (Variables|Default|GetPlayerActions))) Index)))
    (Default|AddGridTile (Variables|/Game/TurnBasedTactic/Blueprints/Core/Player/BP_PlayerActions.BP_PlayerActions_C|GetGrid (Variables|Default|GetPlayerActions)) (Utilities|Struct|MakeS_TileData (.Index (Utilities|Struct|BreakS_TileData (LocalVariables|GetData))) (.Type (Utilities|Struct|BreakS_TileData (LocalVariables|GetData))) (Math|Transform|MakeTransform (+ (.Location (Math|Transform|BreakTransform (.Transform (Utilities|Struct|BreakS_TileData (LocalVariables|GetData))))) (Math|Vector|MakeVector 0.0 0.0 (* (.z (Variables|/Game/TurnBasedTactic/Blueprints/Core/Grid/BP_Grid.BP_Grid_C|GetGridTileSize (Variables|/Game/TurnBasedTactic/Blueprints/Core/Player/BP_PlayerActions.BP_PlayerActions_C|GetGrid (Variables|Default|GetPlayerActions)))) (Math|Float|SelectFloat 1.0 -1.0 (Variables|Default|GetIncrease))))) (.Rotation (Math|Transform|BreakTransform (.Transform (Utilities|Struct|BreakS_TileData (LocalVariables|GetData))))) (.Scale (Math|Transform|BreakTransform (.Transform (Utilities|Struct|BreakS_TileData (LocalVariables|GetData)))))) (.States (Utilities|Struct|BreakS_TileData (LocalVariables|GetData))) (.UnitOnTile (Utilities|Struct|BreakS_TileData (LocalVariables|GetData)))))))