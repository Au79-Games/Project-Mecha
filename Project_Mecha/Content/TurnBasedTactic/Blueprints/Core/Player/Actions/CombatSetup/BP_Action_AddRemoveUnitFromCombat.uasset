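; Player action that adds or removes a combat unit on a grid tile during combat setup.
; When adding, it first checks that the tile type is valid for the chosen unit type, then removes and destroys any occupant.
; It then spawns a BP_Unit and registers it with the CombatSystem using the team index and AI flag.
; When removing, it reuses the same removal path.
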(event EventBeginPlay
  (|CallParentFunction) ; This node is disabled and will not be called.\nDrag off pins to build functionality.
)

(event Collision|EventActorBeginOverlap
  (params (OtherActor :type Actor%20Object%20Reference))
  (|CallParentFunction OtherActor) ; This node is disabled and will not be called.\nDrag off pins to build functionality.
)

(event EventTick
  (params (DeltaSeconds :type Float%20%28single-precision%29))
  (|CallParentFunction DeltaSeconds) ; This node is disabled and will not be called.\nDrag off pins to build functionality.
)

(fn ConstructionScript
  (|CallParentFunction))

(fn ExecuteAction
  (params (Index :type Int%20Point%20Structure))
  ;[0 0 0] [EN] When we add a unit, we first make sure to remove the previous unit (if valid) and then we can spawn the new unit and place it on the grid.
  ; [FR] Quand on ajoute une unité, on fait d'abbord sûr d'enlever l'unité déjà présente sur la case (si valide) et ensuite on peut spawn notre nouvelle unité et la placer sur la grille
  (if (Variables|Default|GetIsAddingUnit)
    (bind _unitdata (CallFunction|GetDefaultUnitDatafromUnitType (Variables|Default|GetUnitType)))
    (if (Utilities|Array|ContainsItem (.ValidTileTypes (Utilities|Struct|BreakS_UnitData_Stats (.Stats (Utilities|Struct|BreakS_UnitData _unitdata)))) (.Type (Utilities|Struct|BreakS_TileData (.Value (Utilities|Map|Find (Variables|/Game/TurnBasedTactic/Blueprints/Core/Grid/BP_Grid.BP_Grid_C|GetGridTiles (Variables|/Game/TurnBasedTactic/Blueprints/Core/Player/BP_PlayerActions.BP_PlayerActions_C|GetGrid (Variables|Default|GetPlayerActions))) Index)))))
      (Utilities|FlowControl|Sequence
        (:then_0
          (bind _output_get (LocalVariables|SetUnit (Utilities|Struct|BreakS_TileData (.Value (Utilities|Map|Find (Variables|/Game/TurnBasedTactic/Blueprints/Core/Grid/BP_Grid.BP_Grid_C|GetGridTiles (Variables|/Game/TurnBasedTactic/Blueprints/Core/Player/BP_PlayerActions.BP_PlayerActions_C|GetGrid (Variables|Default|GetPlayerActions))) Index))) :!label _label))
          (Utilities|IsValid _output_get
            (:Is%20Valid
              (Default|RemoveUnitfromCombat (Variables|/Game/TurnBasedTactic/Blueprints/Core/Player/BP_PlayerActions.BP_PlayerActions_C|GetCombatSystem (Variables|Default|GetPlayerActions)) (LocalVariables|GetUnit))
              (Actor|DestroyActor (LocalVariables|GetUnit)))))
        (:then_1
          (bind _returnvalue (Game|SpawnActorfromClass "/Game/TurnBasedTactic/Blueprints/Core/Units/BP_Unit.BP_Unit_C" (Math|Transform|MakeTransform "0, 0, 0" "0, 0, 0" "1.000000,1.000000,1.000000") "AlwaysSpawn" "MultiplyWithRoot" 0 (Variables|Default|GetUnitType) 0))
          (Default|AddUnitinCombat (Variables|/Game/TurnBasedTactic/Blueprints/Core/Player/BP_PlayerActions.BP_PlayerActions_C|GetCombatSystem (Variables|Default|GetPlayerActions)) _returnvalue Index (Variables|Default|GetTeamIndex) (Variables|Default|GetUseAi)))))
    (else
      (goto _label))))